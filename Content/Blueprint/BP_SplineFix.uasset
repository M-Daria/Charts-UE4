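; BP_SplineFix is a spline-driven pipe actor that builds a pipe from repeated mesh segments along its spline.
; The construction script divides the spline length by SectionLength and adds a spline mesh component per section with the configured mesh, material and uniform cross-section scale.
; Each segment takes local-space positions and tangents at its boundary distances, with tangent lengths clamped to the section length.
; The event graph holds no runtime logic.
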(event EventBeginPlay)

(event Collision|EventActorBeginOverlap
  (params (OtherActor :type Actor%20Object%20Reference)))

(event EventTick
  (params (DeltaSeconds :type Float%20%28single-precision%29)))

(fn ConstructionScript
  (bind _scale (Variables|Default|GetScale))
  (bind _spline (Variables|Default|GetSpline))
  (bind _sectionlength (Variables|Default|GetSectionLength))
  (for _index (range 0 (Math|Float|Truncate (/ (Spline|GetSplineLength (Variables|Default|GetSpline)) (Variables|Default|GetSectionLength))))
    (bind _returnvalue (AddComponent|AddSplineMeshComponent false))
    (Components|StaticMesh|SetStaticMesh _returnvalue (Variables|Default|GetPipeMesh))
    (Rendering|Material|SetMaterial _returnvalue 0 (Variables|Default|GetPipeMaterial))
    (SplineMesh|SetStartScale _returnvalue (Math|Vector2D|MakeVector2D _scale _scale) true :!class /Script/Engine.SplineMeshComponent)
    (SplineMesh|SetEndScale _returnvalue (Math|Vector2D|MakeVector2D _scale _scale) true :!class /Script/Engine.SplineMeshComponent)
    (SplineMesh|SetStartandEnd _returnvalue (Spline|GetLocationatDistanceAlongSpline _spline (* _index _sectionlength) "Local") (Math|Vector|ClampVectorSize (Spline|GetTangentatDistanceAlongSpline _spline (* _index _sectionlength) "Local") 0.0 (Variables|Default|GetSectionLength)) (Spline|GetLocationatDistanceAlongSpline _spline (* (+ _index 1) _sectionlength) "Local") (Math|Vector|ClampVectorSize (Spline|GetTangentatDistanceAlongSpline _spline (* (+ _index 1) _sectionlength) "Local") 0.0 (Variables|Default|GetSectionLength)) true :!class /Script/Engine.SplineMeshComponent)))