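; Test Blueprint that builds a "Random values" line chart through a ChartView, entirely in the construction script.
; It fills an array with random Y values over a symmetric integer X range and plots it as a dotted line alongside a fixed, sloped dashed line.
; A sequence then sets autoscaled axes, viewport size, colors, grid and title.
; The axis label calls are unconnected, and the event graph is empty.
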(event EventBeginPlay)

(event Collision|EventActorBeginOverlap
  (params (OtherActor :type Actor%20Object%20Reference)))

(event EventTick
  (params (DeltaSeconds :type Float%20%28single-precision%29)))

(fn ConstructionScript
  (bind _array (LocalVariables|Getarray))
  (bind _chartview (Variables|Default|GetChartView))
  (bind _chartview_2 (Variables|Default|GetChartView))
  (bind _chartview_3 (Variables|Default|GetChartView))
  (bind _chartview_4 (Variables|Default|GetChartView))
  (Utilities|FlowControl|Sequence
    (:then_0
      (for _index (range -25 25)
        (Utilities|Array|Add _array (Math|Vector2D|MakeVector2D (Math|Conversions|ToFloat(Integer) _index) (Math|Random|RandomFloat)))))
    (:then_1
      (Class|ChartViewComponent|CreateChartViewport _chartview)
      (Class|ChartViewComponent|AddLine _chartview 1 _array)
      (Class|ChartViewComponent|AddLine _chartview 0 (Utilities|Array|MakeArray "(X=-25.000000,Y=0.200000)" "(X=25.000000,Y=0.800000)"))
      (Class|ChartViewComponent|SetXRange _chartview_2 (Math|Vector2D|MakeVector2D 0.0 1e+03))
      (Class|ChartViewComponent|SetYRange _chartview_2 (Math|Vector2D|MakeVector2D 0.0 2.0))
      (Class|ChartViewComponent|SetXAutoscale _chartview_2 true)
      (Class|ChartViewComponent|SetYAutoscale _chartview_2 true)
      (Class|ChartViewComponent|SetViewportSize _chartview_2 (Math|Vector2D|MakeVector2D 4e+02 5e+02)))
    (:then_2
      (Class|ChartViewComponent|SetLineColor _chartview_3 0 (Math|Conversions|ToLinearColor(Color) (Math|Conversions|ToColor(LinearColor) "(R=0.011425,G=0.000000,B=0.120833,A=1.000000)")))
      (Class|ChartViewComponent|SetLineColor _chartview_3 1 (Math|Conversions|ToLinearColor(Color) (Math|Conversions|ToColor(LinearColor) "(R=0.120833,G=0.000000,B=0.029587,A=1.000000)")))
      (Class|ChartViewComponent|SetLineType _chartview_3 0 "Dashed")
      (Class|ChartViewComponent|SetLineType _chartview_3 1 "Dotted")
      (Class|ChartViewComponent|SetLineDashInterval _chartview_3 0 5.0)
      (Class|ChartViewComponent|SetLineDashLength _chartview_3 0 8.0)
      (Class|ChartViewComponent|SetLineWidth _chartview_3 0 2.0)
      (Class|ChartViewComponent|SetLineWidth _chartview_3 1 3.0)
      (Class|ChartViewComponent|SetChartBackgroundColor _chartview_4 (Math|Conversions|ToLinearColor(Color) (Math|Conversions|ToColor(LinearColor) "(R=0.443464,G=0.516667,B=0.495801,A=1.000000)")))
      (Class|ChartViewComponent|SetChartGridColor _chartview_4 (Math|Conversions|ToLinearColor(Color) (Math|Conversions|ToColor(LinearColor) "(R=0.229167,G=0.229167,B=0.229167,A=1.000000)")))
      (Class|ChartViewComponent|SetChartGridType _chartview_4 "Solid")
      (Class|ChartViewComponent|SetTextColor _chartview_4 "Title" (Math|Conversions|ToColor(LinearColor) "(R=0.010353,G=0.000000,B=0.166667,A=1.000000)"))
      (Class|ChartViewComponent|SetTextSize _chartview_4 "Title" 4e+01)
      (Class|ChartViewComponent|SetTextTitle _chartview_4 (Utilities|Text|MakeLiteralText "Random values")))))