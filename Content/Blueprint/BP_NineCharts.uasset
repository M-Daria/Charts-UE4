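; BP_NineCharts is a display actor showing a 3x3 dashboard of brand tiles, each with an icon, dollar figure and line chart.
; The construction script lays out procedural-mesh quads for icons, tile backgrounds and backdrop, with gradient UVs spanning the grid.
; Each tile adds a TextRender and a ChartView component filled with random placeholder data, regenerated on every construction run.
; BeginPlay creates one additional, unconfigured chart viewport.
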(event EventBeginPlay
  (bind _returnvalue (AddComponent|AddChartViewComponent false))
  (Class|ChartViewComponent|CreateChartViewport _returnvalue))

(event Collision|EventActorBeginOverlap
  (params (OtherActor :type Actor%20Object%20Reference)))

(event EventTick
  (params (DeltaSeconds :type Float%20%28single-precision%29)))

(fn ConstructionScript
  (bind _returnvalue (Math|Integer|%(Integer) 8 -3))
  (bind _returnvalue_2 (/ 8 3))
  (bind _background_charts_width (LocalVariables|GetBackground%20Charts%20Width))
  (bind _background_charts_height (LocalVariables|GetBackground%20Charts%20Height))
  (bind _icon_width (LocalVariables|GetIcon%20Width))
  (bind _arrayofvalues (LocalVariables|GetArrayOfValues))
  (bind _background (Variables|Default|GetBackground))
  (bind _backgroundcharts (Variables|Default|GetBackgroundCharts))
  (bind _returnvalue_3 (* _returnvalue_2 5e+02))
  (bind _returnvalue_4 (* _returnvalue 6e+02))
  (bind _returnvalue_5 (+ _returnvalue_4 _background_charts_width))
  (bind _returnvalue_6 (+ _returnvalue_3 _background_charts_height))
  (for _index (range 0 8)
    ;[1 1 1] Icons
    (Class|ProceduralMeshComponent|CreateMeshSectionLinearColor (Variables|Default|GetIcons) _index (Utilities|Array|MakeArray (Math|Vector|MakeVector (+ (* (Math|Integer|%(Integer) _index -3) 7e+02) (LocalVariables|GetShift%20Icon%20X)) 0.01 (+ (* (/ _index 3) 5e+02) (- (- (LocalVariables|GetBackground%20Charts%20Height) (LocalVariables|GetShift%20Icon%20Y)) _icon_width))) (Math|Vector|MakeVector (+ (* (Math|Integer|%(Integer) _index -3) 7e+02) (LocalVariables|GetShift%20Icon%20X)) 0.01 (+ (+ (* (/ _index 3) 5e+02) (- (- (LocalVariables|GetBackground%20Charts%20Height) (LocalVariables|GetShift%20Icon%20Y)) _icon_width)) _icon_width)) (Math|Vector|MakeVector (+ (+ (* (Math|Integer|%(Integer) _index -3) 7e+02) (LocalVariables|GetShift%20Icon%20X)) (LocalVariables|GetIcon%20Width)) 0.01 (+ (* (/ _index 3) 5e+02) (- (- (LocalVariables|GetBackground%20Charts%20Height) (LocalVariables|GetShift%20Icon%20Y)) _icon_width))) (Math|Vector|MakeVector (+ (+ (* (Math|Integer|%(Integer) _index -3) 7e+02) (LocalVariables|GetShift%20Icon%20X)) (LocalVariables|GetIcon%20Width)) 0.01 (+ (+ (* (/ _index 3) 5e+02) (- (- (LocalVariables|GetBackground%20Charts%20Height) (LocalVariables|GetShift%20Icon%20Y)) _icon_width)) _icon_width))) (LocalVariables|GetQuad%20Tri) 0 (LocalVariables|GetIcons%20UV) 0 0 0 0 0 false)
    (Rendering|Material|CreateDynamicMaterialInstance (Variables|Default|GetIcons) _index (Utilities|Array|Get(acopy) (LocalVariables|GetIcon%20Dyn%20Materials) _index) "None" :!class /Script/Engine.PrimitiveComponent)
    ;[1 1 1] Charts Back
    (Class|ProceduralMeshComponent|CreateMeshSectionLinearColor _backgroundcharts _index (Utilities|Array|MakeArray (Math|Vector|MakeVector (* (Math|Integer|%(Integer) _index -3) 7e+02) 0.0 (* (/ _index 3) 5e+02)) (Math|Vector|MakeVector (* (Math|Integer|%(Integer) _index -3) 7e+02) 0.0 (+ (* (/ _index 3) 5e+02) (LocalVariables|GetBackground%20Charts%20Height))) (Math|Vector|MakeVector (+ (* (Math|Integer|%(Integer) _index -3) 7e+02) (LocalVariables|GetBackground%20Charts%20Width)) 0.0 (* (/ _index 3) 5e+02)) (Math|Vector|MakeVector (+ (* (Math|Integer|%(Integer) _index -3) 7e+02) (LocalVariables|GetBackground%20Charts%20Width)) 0.0 (+ (* (/ _index 3) 5e+02) (LocalVariables|GetBackground%20Charts%20Height)))) (LocalVariables|GetQuad%20Tri) 0 (Utilities|Array|MakeArray (Math|Vector2D|MakeVector2D (/ (* (Math|Integer|%(Integer) _index -3) 7e+02) _returnvalue_5) (/ (* (/ _index 3) 5e+02) _returnvalue_6)) (Math|Vector2D|MakeVector2D (/ (* (Math|Integer|%(Integer) _index -3) 7e+02) _returnvalue_5) (/ (+ (* (/ _index 3) 5e+02) (LocalVariables|GetBackground%20Charts%20Height)) _returnvalue_6)) (Math|Vector2D|MakeVector2D (/ (+ (* (Math|Integer|%(Integer) _index -3) 7e+02) (LocalVariables|GetBackground%20Charts%20Width)) _returnvalue_5) (/ (* (/ _index 3) 5e+02) _returnvalue_6)) (Math|Vector2D|MakeVector2D (/ (+ (* (Math|Integer|%(Integer) _index -3) 7e+02) (LocalVariables|GetBackground%20Charts%20Width)) _returnvalue_5) (/ (+ (* (/ _index 3) 5e+02) (LocalVariables|GetBackground%20Charts%20Height)) _returnvalue_6))) 0 0 0 0 0 false)
    (Rendering|Material|CreateDynamicMaterialInstance _backgroundcharts _index "/Game/Materials/M_Gradient.M_Gradient" "None" :!class /Script/Engine.PrimitiveComponent)
    ;[1 1 1] Text
    (bind _returnvalue_7 (AddComponent|AddTextRenderComponent false (Math|Transform|MakeTransform (Math|Vector|MakeVector (+ (+ (* (Math|Integer|%(Integer) _index -3) 7e+02) (LocalVariables|GetShift%20Icon%20X)) (/ (LocalVariables|GetIcon%20Width) 2.0)) 0.01 (- (+ (* (/ _index 3) 5e+02) (- (- (LocalVariables|GetBackground%20Charts%20Height) (LocalVariables|GetShift%20Icon%20Y)) _icon_width)) (LocalVariables|GetText%20Offset))) "0.000000,90.000000, 0" "1,1,1")))
    (Rendering|Components|TextRender|SetText _returnvalue_7 (Utilities|Text|ToText(String) (Utilities|String|Append (Utilities|String|ToString(Text) (Utilities|Text|ToText(Float) (Math|Random|RandomFloatinRange -6e+02 6e+02) "HalfToEven" true true 1 324 0 2)) "$")))
    (Class|TextRenderComponent|SetVerticalAlignment _returnvalue_7 "EVRTA_TextTop")
    (Rendering|Components|TextRender|SetHorizontalAlignment _returnvalue_7 "EHTA_Center")
    ;[1 1 1] Chart
    (bind _returnvalue_8 (AddComponent|AddChartViewComponent false (Math|Transform|MakeTransform (Math|Vector|MakeVector (+ (* (Math|Integer|%(Integer) _index -3) 7e+02) (- (- (LocalVariables|GetBackground%20Charts%20Width) (LocalVariables|GetChart%20Width)) (LocalVariables|GetChart%20Offset%20X))) 0.01 (+ (* (/ _index 3) 5e+02) (- (- (LocalVariables|GetBackground%20Charts%20Height) (LocalVariables|GetChart%20Height)) (LocalVariables|GetChart%20Offset%20Y)))) "0, 0, 0" "1,1,1")))
    (Class|ChartViewComponent|CreateChartViewport _returnvalue_8)
    (Class|ChartViewComponent|SetViewportSize _returnvalue_8 (Math|Vector2D|MakeVector2D (LocalVariables|GetChart%20Width) (LocalVariables|GetChart%20Height)))
    (Class|ChartViewComponent|SetTextTitle _returnvalue_8 (Utilities|Array|Get(acopy) (LocalVariables|GetBrands%20Name) _index))
    (Class|ChartViewComponent|SetTextSize _returnvalue_8 "Title" 5e+01)
    (Class|ChartViewComponent|SetTextColor _returnvalue_8 "Title" (Math|Conversions|ToColor(LinearColor) "(R=0.583333,G=0.583333,B=0.583333,A=1.000000)"))
    (Class|ChartViewComponent|SetTextColor _returnvalue_8 "AxisValues" (Math|Conversions|ToColor(LinearColor) "(R=0.107500,G=0.109063,B=0.200000,A=1.000000)"))
    (Class|ChartViewComponent|SetChartBackgroundColor _returnvalue_8 (Math|Conversions|ToLinearColor(Color) (Math|Conversions|ToColor(LinearColor) "(R=0.000000,G=0.000000,B=0.023529,A=1.000000)")))
    (Class|ChartViewComponent|SetChartGridType _returnvalue_8 "StripedVertical")
    (Class|ChartViewComponent|SetChartGridColor _returnvalue_8 (Math|Conversions|ToLinearColor(Color) (Math|Conversions|ToColor(LinearColor) "(R=0.000000,G=0.000000,B=0.008333,A=1.000000)")))
    (for _index_2 (range 0 25)
      (Utilities|Array|Add (LocalVariables|GetArrayOfValues) (Math|Vector2D|MakeVector2D (Math|Float|MapRangeClamped (Math|Conversions|ToFloat(Integer) _index_2) 0.0 25.0 0.0 1.5e+02) (Math|Random|RandomFloatinRange 0.0 15.0))))
    (Class|ChartViewComponent|AddLine _returnvalue_8 _index _arrayofvalues)
    (Utilities|Array|Clear _arrayofvalues)
    (Class|ChartViewComponent|SetLineWidth _returnvalue_8 _index 2.0)
    (Class|ChartViewComponent|SetYRange _returnvalue_8 (Math|Vector2D|MakeVector2D 0.0 15.0)))
  (Class|ProceduralMeshComponent|CreateMeshSectionLinearColor _background 0 (Utilities|Array|MakeArray "-25.000000,-0.01,-25.000000" "-25.000000,-0.010000,1500.000000" "2100.000000,-0.010000,-25.000000" "2100.000000,-0.010000,1500.000000") (LocalVariables|GetQuad%20Tri) 0 (Utilities|Array|MakeArray "(X=1.000000,Y=1.000000)" "(X=1.000000,Y=0.000000)" "(X=0.000000,Y=1.000000)" "(X=0.000000,Y=0.000000)") 0 0 0 0 0 false)
  (bind _returnvalue_9 (Rendering|Material|CreateDynamicMaterialInstance _background 0 "/Game/Materials/M_Gradient.M_Gradient" "None" :!class /Script/Engine.PrimitiveComponent))
  (Rendering|Material|SetVectorParameterValue _returnvalue_9 "Base Color Bottom" "(R=0.006290,G=0.000000,B=0.304167,A=1.000000)" :!class /Script/Engine.MaterialInstanceDynamic)
  (Rendering|Material|SetVectorParameterValue :self _returnvalue_9 :ParameterName "Base Color Top" :!class /Script/Engine.MaterialInstanceDynamic))