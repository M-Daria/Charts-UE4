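; Test Blueprint that draws a sample "Random values" line chart from two hardcoded point sets through its ChartView.
; The Construction Script builds the point arrays, creates the chart viewport, adds both lines and enables autoscaling on both axes after setting ranges.
; It then styles lines, background, dashed grid and title.
; The axis label calls are disconnected, and the Event Graph is empty.
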(event EventBeginPlay)

(event Collision|EventActorBeginOverlap
  (params (OtherActor :type Actor%20Object%20Reference)))

(event EventTick
  (params (DeltaSeconds :type Float%20%28single-precision%29)))

(fn ConstructionScript
  (bind _returnvalue (Math|Conversions|ToColor(LinearColor) "(R=0.000000,G=0.000000,B=0.000000,A=1.000000)"))
  (bind _chartview (Variables|Default|GetChartView))
  (bind _chartview_2 (Variables|Default|GetChartView))
  (bind _chartview_3 (Variables|Default|GetChartView))
  (bind _chartview_4 (Variables|Default|GetChartView))
  (Utilities|FlowControl|Sequence
    (:then_0
      (LocalVariables|Setarray (Utilities|Array|MakeArray "(X=-50.000000,Y=50.000000)" "(X=-40.000000,Y=2.000000)" "(X=-30.000000,Y=25.000000)" "(X=-20.000000,Y=10.000000)" "(X=-10.000000,Y=15.000000)"))
      (Utilities|Array|AppendArray (LocalVariables|Getarray) (Utilities|Array|MakeArray "" "(X=20.000000,Y=20.000000)" "(X=30.000000,Y=55.000000)" "(X=50.000000,Y=90.000000)" "(X=80.000000,Y=54.000000)" "(X=90.000000,Y=45.000000)" "(X=100.000000,Y=24.000000)" "(X=110.000000,Y=40.000000)" "(X=120.000000,Y=25.000000)" "(X=130.000000,Y=-7.000000)" "(X=140.000000,Y=-13.000000)" "(X=150.000000,Y=27.000000)" "(X=160.000000,Y=25.000000)" "(X=170.000000,Y=69.000000)" "(X=180.000000,Y=30.000000)" "(X=190.000000,Y=22.000000)"))
      (LocalVariables|Setarray_0 (Utilities|Array|MakeArray "(X=-80.000000,Y=0.000000)" "(X=-70.000000,Y=0.000000)" "(X=-65.000000,Y=20.000000)"))
      (Utilities|Array|AppendArray (LocalVariables|Getarray_0) (Utilities|Array|MakeArray "(X=-60.000000,Y=-10.000000)" "(X=-30.000000,Y=20.000000)" "(X=2.000000,Y=40.000000)" "(X=80.000000,Y=80.000000)" "(X=90.000000,Y=33.000000)" "(X=100.000000,Y=24.000000)" "(X=120.000000,Y=-2.000000)" "(X=140.000000,Y=0.000000)" "(X=150.000000,Y=32.000000)" "(X=160.000000,Y=0.000000)" "(X=170.000000,Y=22.000000)")))
    (:then_1
      (Class|ChartViewComponent|CreateChartViewport _chartview)
      (Class|ChartViewComponent|AddLine _chartview 1 (LocalVariables|Getarray))
      (Class|ChartViewComponent|AddLine _chartview 0 (LocalVariables|Getarray_0))
      (Class|ChartViewComponent|SetXRange _chartview_2 (Math|Vector2D|MakeVector2D 0.0 1e+03))
      (Class|ChartViewComponent|SetYRange _chartview_2 (Math|Vector2D|MakeVector2D 0.0 2.0))
      (Class|ChartViewComponent|SetXAutoscale _chartview_2 true)
      (Class|ChartViewComponent|SetYAutoscale _chartview_2 true)
      (Class|ChartViewComponent|SetViewportSize _chartview_2 (Math|Vector2D|MakeVector2D 6e+02 4e+02)))
    (:then_2
      (Class|ChartViewComponent|SetLineColor _chartview_3 0 (Math|Conversions|ToLinearColor(Color) (Math|Conversions|ToColor(LinearColor) "(R=0.223432,G=0.000000,B=1.000000,A=1.000000)")))
      (Class|ChartViewComponent|SetLineColor _chartview_3 1 (Math|Conversions|ToLinearColor(Color) (Math|Conversions|ToColor(LinearColor) "(R=1.000000,G=0.437420,B=0.000000,A=1.000000)")))
      (Class|ChartViewComponent|SetLineType _chartview_3 0 "Solid")
      (Class|ChartViewComponent|SetLineType _chartview_3 1 "Solid")
      (Class|ChartViewComponent|SetLineDashInterval _chartview_3 0 5.0)
      (Class|ChartViewComponent|SetLineDashLength _chartview_3 0 8.0)
      (Class|ChartViewComponent|SetLineWidth _chartview_3 0 2.0)
      (Class|ChartViewComponent|SetLineWidth _chartview_3 1 2.0)
      (Class|ChartViewComponent|SetChartBackgroundColor _chartview_4 (Math|Conversions|ToLinearColor(Color) (Math|Conversions|ToColor(LinearColor) "(R=0.000000,G=0.000000,B=0.000000,A=1.000000)")))
      (Class|ChartViewComponent|SetChartGridColor _chartview_4 (Math|Conversions|ToLinearColor(Color) (Math|Conversions|ToColor(LinearColor) "(R=0.028333,G=0.197980,B=0.212500,A=1.000000)")))
      (Class|ChartViewComponent|SetChartGridType _chartview_4 "Dashed")
      (Class|ChartViewComponent|SetTextColor _chartview_4 "Title" _returnvalue)
      (Class|ChartViewComponent|SetTextColor _chartview_4 "AxisValues" _returnvalue)
      (Class|ChartViewComponent|SetTextSize _chartview_4 "Title" 4e+01)
      (Class|ChartViewComponent|SetTextTitle _chartview_4 (Utilities|Text|MakeLiteralText "Random values")))))